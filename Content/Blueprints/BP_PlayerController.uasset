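; Player controller for a pinball game that routes player input to the table's flippers and plunger.
; On BeginPlay it finds all Flipper actors, sorting them into left and right arrays by FlipType, caches the first BP_Plugger as the plunger, and creates the PinballHUD widget.
; Left and right flip inputs call Flip and Flop on every flipper of that side, while Charge press and release charge and fire the plunger.
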(event Custom|DetectFlipper
  (bind _outactors (Actor|GetAllActorsOfClass "/Game/Blueprints/Flipper.Flipper_C"))
  (for _array_element _outactors
    (switch Utilities|FlowControl|Switch|SwitchonFlipperType (Variables|/Game/Blueprints/Flipper.Flipper_C|GetFlipType _array_element)
      (:NewEnumerator0
        (Utilities|Array|Add (Variables|Default|GetLeftFlipper) _array_element))
      (:NewEnumerator1
        (Utilities|Array|Add (Variables|Default|GetRightFlipper) _array_element)))))

(event Custom|CreatePlayerHUD
  (Viewport|RemoveAllWidgets)
  (bind _returnvalue (UserInterface|CreateWidget "/Game/Blueprints/PinballHud.PinballHUD_C"))
  (UserInterface|Viewport|AddtoViewport _returnvalue 0))

(event Custom|DetectPlunger
  (bind _outactors (Actor|GetAllActorsOfClass "/Game/Blueprints/BP_Plugger.BP_Plugger_C"))
  (Variables|Default|SetPlunger (Utilities|Array|Get(acopy) _outactors)))

(event EventBeginPlay
  (CallFunction|DetectFlipper)
  (CallFunction|DetectPlunger)
  (CallFunction|CreatePlayerHUD))

(event EventTick
  (params (DeltaSeconds :type Float%20%28single-precision%29)))

(event Input|ActionEvents|InputActionCharge
  (params (Key :type Key%20Structure :default "AnyKey"))
  (bind _plunger (Variables|Default|GetPlunger))
  (:Pressed
    (Default|ChargePlunger _plunger))
  (:Released
    (Default|ReleasePlunger _plunger)))

(event Input|ActionEvents|InputActionRightFlip
  (params (Key :type Key%20Structure :default "AnyKey"))
  (bind _rightflipper (Variables|Default|GetRightFlipper))
  (:Pressed
    (for _array_element _rightflipper
      (Default|Flip _array_element)))
  (:Released
    (for _array_element_2 _rightflipper
      (Default|Flop _array_element_2))))

(event Input|ActionEvents|InputActionLeftFlip
  (params (Key :type Key%20Structure :default "AnyKey"))
  (bind _leftflipper (Variables|Default|GetLeftFlipper))
  (:Pressed
    (for _array_element _leftflipper
      (Default|Flip _array_element)))
  (:Released
    (for _array_element_2 _leftflipper
      (Default|Flop _array_element_2))))

(fn ConstructionScript)